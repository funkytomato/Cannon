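; Actor component that drives an auto-targeting turret on BP_NewCannon.
; On BeginPlay it loads gun and munition stats from DT_Guns and DT_Munitions, then seeds its target list from the detection sphere after a short delay.
; Looping timers interp the turret toward the first detected target and spawn projectiles while the focus collision overlaps a target.
; Fire interval and interp speed are hardcoded, ignoring the loaded FireRate and TurretRotationSpeed.
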(event `self.ReceiveBeginPlay`
  (bind _asbp_new_cannon (cast `/Game/MyContent/Blueprints/Cannon/BP_NewCannon` (`self.GetOwner`)))
  (set `self.MyCannonRef` _asbp_new_cannon)
  (`|ExecutionSequence`
    (:`then_0`
      ;[1 1 1] Load Gun Characteristics
      (bind _returnvalue (`|GetDataTableRow` "/Game/MyContent/Blueprints/Cannon/DT_Guns.DT_Guns" (`KismetStringLibrary.Conv_StringToName` (`|GetEnumeratorNameAsString` (`/Game/MyContent/Blueprints/Cannon/BP_NewCannon.GunType` (`self.MyCannonRef`)))))
        (:`then`
          (bind (_gunname _firetype _firerate _reloadtime _reloadsfx _firefx _aimtype _turretrotationspeed _turretrotationsfx _turretelevationspeed) (break `/Game/MyContent/Blueprints/Cannon/S_GunCharacteristics` _returnvalue))
          (set `self.GunName` _gunname)
          (set `self.FireType` _firetype)
          (set `self.FireRate` _firerate)
          (set `self.ReloadTime` _reloadtime)
          (set `self.ReloadSFX` _reloadsfx)
          (set `self.FireFX` _firefx)
          (set `self.AimType` _aimtype)
          (set `self.TurretRotationSpeed` _turretrotationspeed)
          (set `self.TurretRotationSFX` _turretrotationsfx)
          (set `self.TurretElevationSpeed` _turretelevationspeed)
          ;[1 1 1] Munition Properties
          (bind _returnvalue_2 (`|GetDataTableRow` "/Game/MyContent/Blueprints/Cannon/DT_Munitions.DT_Munitions" (`KismetStringLibrary.Conv_StringToName` (`|GetEnumeratorNameAsString` (`/Game/MyContent/Blueprints/Cannon/BP_NewCannon.MuntionType` (`self.MyCannonRef`)))))
            (:`then`
              (bind (_muntionname _damagetype _munitionclass _hitfx _hitsfx _projectilespeed) (break `/Game/MyContent/Blueprints/Cannon/S_Munition` _returnvalue_2))
              (set `self.MunitionName` _muntionname)
              (set `self.DamageType` _damagetype)
              (set `self.MunitionClass` _munitionclass)
              (set `self.HitFX` _hitfx)
              (set `self.HitSFX` _hitsfx)
              (set `self.Projectile Speed` _projectilespeed))))))
    (:`then_1`
      ;[1 1 1] Configure Timers for Turret Articulation and Firing Sequence
      (`KismetSystemLibrary.K2_SetTimer` null "FocusOnTarget" 0.05 true)
      (`KismetSystemLibrary.K2_SetTimer` null "Fire" 1.0 true))
    (:`then_2`
      ;[1 1 1] Detect for any Targets within Detection Sphere at beginning of the game
      (`KismetSystemLibrary.Delay` 1.0)
      (for _array_element (`PrimitiveComponent.GetOverlappingActors` (`/Game/MyContent/Blueprints/Cannon/BP_NewCannon.DetectionSphere` (`self.MyCannonRef`)) (`/Game/MyContent/Blueprints/Cannon/BP_NewCannon.TargetType` (`self.MyCannonRef`)))
        (`self.CheckDetectedTargetAndAdd` _array_element)))))

(event `StartShooting`
  ;[1 1 1] Shooting - Start and Stop
  (set `self.IsShooting` true))

(event `StopShooting`
  ;[1 1 1] Shooting - Start and Stop
  (set `self.IsShooting` false))

(fn `CheckDetectedTargetAndAdd`
  (params (Target :type "Actor Object Reference"))
  (if (== (`GameplayStatics.GetObjectClass` Target) (`/Game/MyContent/Blueprints/Cannon/BP_NewCannon.TargetType` (`self.MyCannonRef`)))
    (`KismetArrayLibrary.Array_AddUnique` (`self.DetectedActors`) Target)))

(fn `Fire`
  (bind (_returnvalue_location _returnvalue_rotation) (`KismetMathLibrary.BreakTransform` (`SceneComponent.K2_GetComponentToWorld` (`/Game/MyContent/Blueprints/Cannon/BP_NewCannon.ProjectileSpawnPoint` (`self.MyCannonRef`)))))
  (if (`self.IsShooting`)
    (bind _focused (`self.TurretFocusedOnTarget`))
    (if _focused
      (`|SpawnActorFromClass` (`self.MunitionClass`) (`KismetMathLibrary.MakeTransform` _returnvalue_location _returnvalue_rotation) "AlwaysSpawn" "MultiplyWithRoot" (`self.MyCannonRef`) (`self.HitFX`) (`self.HitSFX`) (`self.DamageType`) (`self.Projectile Speed`) null))))

(fn `FocusOnTarget`
  (if (`KismetArrayLibrary.Array_IsNotEmpty` (`self.DetectedActors`))
    (bind _output_get (set `self.CurrentTarget` (`|GetArrayItem` (`self.DetectedActors`))))
    (`self.RotateAndElevateTurret` (`Actor.K2_GetActorLocation` _output_get))
    (`self.StartShooting`)
    (`/Engine/EditorBlueprintResources/StandardMacros.IsValid` (`self.CurrentTarget`)
      (:`Is Not Valid`
        (`self.StopShooting`)
        (return)))))

(fn `PlayAudio`
  (returns (AudioRef :type "AudioComponent Object Reference"))
  (locals (movementSound :type "AudioComponent Object Reference"))
  (bind _returnvalue (`GameplayStatics.SpawnSoundAtLocation` (`self.TurretRotationSFX`) (`SceneComponent.K2_GetComponentLocation` (`Actor.RootComponent` (`self.MyCannonRef`))) (struct) 1.0 1.0 0.0 null null false))
  (bind _output_get (set `local.movementSound` _returnvalue))
  (return _output_get))

(fn `RemoveDetectedTarget`
  (params (Target :type "Actor Object Reference"))
  (returns (Success :type Boolean))
  (bind _returnvalue (`KismetArrayLibrary.Array_RemoveItem` (`self.DetectedActors`) Target))
  (return _returnvalue))

(fn `RotateAndElevateTurret`
  (params (TargetLocation :type "Vector Structure"))
  (bind _mycannonref (`self.MyCannonRef`))
  (bind _returnvalue (`KismetMathLibrary.FindLookAtRotation` (`Actor.K2_GetActorLocation` _mycannonref) (`local.TargetLocation`)))
  (bind (_returnvalue_roll _returnvalue_pitch _returnvalue_yaw) (`KismetMathLibrary.BreakRotator` (`KismetMathLibrary.RInterpTo` (`SceneComponent.K2_GetComponentRotation` (`/Game/MyContent/Blueprints/Cannon/BP_NewCannon.Turret` _mycannonref)) _returnvalue (`GameplayStatics.GetWorldDeltaSeconds`) 5.0)))
  (`SceneComponent.K2_SetWorldRotation` (`/Game/MyContent/Blueprints/Cannon/BP_NewCannon.Turret` (`self.MyCannonRef`)) (`KismetMathLibrary.MakeRotator` 0.0 (`KismetMathLibrary.SelectFloat` _returnvalue_pitch 0.0 (`self.CanElevate?`)) (`KismetMathLibrary.SelectFloat` _returnvalue_yaw 0.0 (`self.CanRotate?`))) false false)
  (`/Engine/EditorBlueprintResources/StandardMacros.IsValid` (`self.TurretRotationSFX`)
    (:`Is Valid`
      (bind _audioref (`self.PlayAudio`))
      (if (== (`KismetMathLibrary.MakeRotator` 0.0 _returnvalue_pitch _returnvalue_yaw) (`KismetMathLibrary.MakeRotator` 0.0 (.pitch _returnvalue) (.yaw _returnvalue)) :`ErrorTolerance` 1.0)
        (`self.StopAudio` _audioref)))
    (:`Is Not Valid`
      _))
  (return))

(fn `StopAudio`
  (params (AudioRef :type "AudioComponent Object Reference"))
  (`AudioComponent.Stop` AudioRef)
  (return))

(fn `TurretFocusedOnTarget`
  (returns (Focused :type Boolean))
  (bind _mycannonref (`self.MyCannonRef`))
  (return (`KismetArrayLibrary.Array_IsNotEmpty` (`PrimitiveComponent.GetOverlappingActors` (`/Game/MyContent/Blueprints/Cannon/BP_NewCannon.TurretFocusCollision` _mycannonref) (`/Game/MyContent/Blueprints/Cannon/BP_NewCannon.TargetType` _mycannonref)))))
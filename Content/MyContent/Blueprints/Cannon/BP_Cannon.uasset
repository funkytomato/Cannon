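; BP_Cannon is an automated cannon that detects targets of a configurable class and fires on them.
; A detection sphere maintains the target list through an initial overlap query and begin/end overlap events, filtered by exact class match.
; Each tick, the first listed target drives BPCannonComponent, which rotates, elevates and shoots.
; The gun and munition name assignments are disconnected from the construction script and never run.
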(event `self.ReceiveBeginPlay`
  ;[1 1 1] BeginPlay - Create list of Potential targets
  (for _array_element (`PrimitiveComponent.GetOverlappingActors` (`self.DetecttionSphere`) (`self.TargetType`))
    (`self.CheckAndAddDetectedTarget` _array_element)
    (`self.StartShooting`)))

(event `self.DetecttionSphere.OnComponentBeginOverlap`
  (params (OverlappedComponent :type "PrimitiveComponent Object Reference") (OtherActor :type "Actor Object Reference") (OtherComp :type "PrimitiveComponent Object Reference") (OtherBodyIndex :type Integer) (bFromSweep :type Boolean) (SweepResult :type "HitResult Structure (by ref)"))
  ;[1 1 1] Update Detected Targets on overlap on DetectionSphere
  (`KismetSystemLibrary.PrintString` "Target detected on overlap")
  (`self.CheckAndAddDetectedTarget` OtherActor))

(event `self.DetecttionSphere.OnComponentEndOverlap`
  (params (OverlappedComponent :type "PrimitiveComponent Object Reference") (OtherActor :type "Actor Object Reference") (OtherComp :type "PrimitiveComponent Object Reference") (OtherBodyIndex :type Integer))
  ;[1 1 1] Update Detected Targets on overlap on DetectionSphere
  (`KismetSystemLibrary.PrintString` "Target removed from end overlap")
  (`KismetArrayLibrary.Array_RemoveItem` (`self.DetectedActors`))
  (if (== OtherActor (`self.CurrentTarget`))
    (set `self.CurrentTarget` null)
    (`/Game/MyContent/Blueprints/Cannon/BP_CannonComponent.StopShooting` (`self.BP_CannonComponent`))))

(event `StartShooting`
  (`/Game/MyContent/Blueprints/Cannon/BP_CannonComponent.StartShooting` (`self.BP_CannonComponent`)))

(event `self.ReceiveTick`
  (params (DeltaSeconds :type "Float (single-precision)"))
  (if (`KismetArrayLibrary.Array_IsNotEmpty` (`self.DetectedActors`))
    (bind _output_get (set `self.CurrentTarget` (`|GetArrayItem` (`self.DetectedActors`))))
    (`/Game/MyContent/Blueprints/Cannon/BP_CannonComponent.RotateAndElevateTurret` (`self.BP_CannonComponent`) (`self.K2_GetActorLocation` _output_get))
    (`/Game/MyContent/Blueprints/Cannon/BP_CannonComponent.StartShooting` (`self.BP_CannonComponent`))
    (`/Engine/EditorBlueprintResources/StandardMacros.IsValid` (`self.CurrentTarget`)
      (:`Is Not Valid`
        (`/Game/MyContent/Blueprints/Cannon/BP_CannonComponent.StopShooting` (`self.BP_CannonComponent`))))))

(fn `CheckAndAddDetectedTarget`
  (params (Target :type "Actor Object Reference"))
  (if (== (`GameplayStatics.GetObjectClass` Target) (`self.TargetType`))
    (`KismetArrayLibrary.Array_AddUnique` (`self.DetectedActors`) Target)))

(fn `UserConstructionScript`)